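; Hexagonal board actor that lays out a grid of hex tiles in its Construction Script, with no runtime logic.
; It scans axial U/V coordinates and keeps those whose hex distance from the origin is less than BoardRadius.
; GetTransformCoordinates converts each pair to a pointy-top position scaled by TileSize for a HexagonTile instance.
; Each tile also gets a small text render label showing its coordinates.
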(event EventBeginPlay)

(event EventActorBeginOverlap
  (params (OtherActor :type Actor%20Object%20Reference)))

(event EventTick
  (params (DeltaSeconds :type Float%20%28single-precision%29)))

(fn ConstructionScript
  (bind _boardradius (Variables|Default|GetBoardRadius))
  (bind _returnvalue (- 0 _boardradius))
  (for _index (range _returnvalue _boardradius)
    (LocalVariables|SetCurrentU _index)
    (for _index_2 (range _returnvalue _boardradius)
      (LocalVariables|SetCurrentV _index_2)
      (if (> _boardradius (Board|GetHexDistance (LocalVariables|GetCurrentU) (LocalVariables|GetCurrentV)))
        (Components|InstancedStaticMesh|AddInstance (Variables|Default|GetHexagonTile) (Math|Conversions|ToTransform(Vector) (Math|Vector|MakeVector (.X (Board|GetTransformCoordinates (LocalVariables|GetCurrentU) (LocalVariables|GetCurrentV))) (.Y (Board|GetTransformCoordinates (LocalVariables|GetCurrentU) (LocalVariables|GetCurrentV))) 0.0)))
        (bind _returnvalue_2 (AddComponent|AddTextRenderComponent false (Math|Transform|MakeTransform (Math|Vector|MakeVector (- (.X (Math|Vector|BreakVector (.Location (Math|Transform|BreakTransform (Math|Conversions|ToTransform(Vector) (Math|Vector|MakeVector (.X (Board|GetTransformCoordinates (LocalVariables|GetCurrentU) (LocalVariables|GetCurrentV))) (.Y (Board|GetTransformCoordinates (LocalVariables|GetCurrentU) (LocalVariables|GetCurrentV))) 0.0)))))) -2.0) (- (.Y (Math|Vector|BreakVector (.Location (Math|Transform|BreakTransform (Math|Conversions|ToTransform(Vector) (Math|Vector|MakeVector (.X (Board|GetTransformCoordinates (LocalVariables|GetCurrentU) (LocalVariables|GetCurrentV))) (.Y (Board|GetTransformCoordinates (LocalVariables|GetCurrentU) (LocalVariables|GetCurrentV))) 0.0)))))) -2.0) 1.0) "90.000000,0.000000,0.000000" (.Scale (Math|Transform|BreakTransform (Math|Conversions|ToTransform(Vector) (Math|Vector|MakeVector (.X (Board|GetTransformCoordinates (LocalVariables|GetCurrentU) (LocalVariables|GetCurrentV))) (.Y (Board|GetTransformCoordinates (LocalVariables|GetCurrentU) (LocalVariables|GetCurrentV))) 0.0)))))))
        (Rendering|Components|TextRender|SetText _returnvalue_2 (Utilities|Text|ToText(String) (Utilities|String|Append "(" (Utilities|String|ToString(Integer) (LocalVariables|GetCurrentU)) "," (Utilities|String|ToString(Integer) (LocalVariables|GetCurrentV)) ")")))
        (Rendering|Components|TextRender|SetXScale _returnvalue_2 0.1)
        (Rendering|Components|TextRender|SetYScale _returnvalue_2 0.1)))))

(fn GetTransformCoordinates
  (params (U :type Integer) (V :type Integer))
  (LocalVariables|Setradius (/ (Variables|Default|GetTileSize) 2))
  (return (* (LocalVariables|Getradius) (* (Math|Float|Sqrt 3.0) (+ (Math|Conversions|ToFloat(Integer) U) (/ (Math|Conversions|ToFloat(Integer) V) 2.0)))) (* (* V (LocalVariables|Getradius)) 1.5)))

(fn GetHexDistance
  (params (U1 :type Integer) (V1 :type Integer) (U2 :type Integer) (V2 :type Integer))
  (bind _returnvalue (- U1 U2))
  (bind _returnvalue_2 (- V1 V2))
  (return (/ (+ (Math|Integer|Absolute(Integer) _returnvalue) (Math|Integer|Absolute(Integer) _returnvalue_2) (Math|Integer|Absolute(Integer) (+ _returnvalue _returnvalue_2))) 2)))